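; Trowel checkpoint for a 2D side-scroller that sets the player's respawn point after being hit three times.
; Each hit on its Box launches the player upward, and a non-looping MultiGate advances the sprite through successive flipbooks.
; The third hit writes the Box's starting X/Z, with Y zeroed, to the character's SpawnJoueur, destroys the collision components, then shows a final flipbook after a delay.
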(event OnComponentHit(Box)
  (params (HitComponent :type Primitive%20Component%20Object%20Reference) (OtherActor :type Actor%20Object%20Reference) (OtherComp :type Primitive%20Component%20Object%20Reference) (NormalImpulse :type Vector :default "0, 0, 0") (Hit :type Hit%20Result%20Structure%20%28by%20ref%29))
  (bind _returnvalue (Game|GetPlayerCharacter 0))
  (bind _respawnpos (Variables|Default|GetRespawnPos))
  (bind _sprite (Variables|Default|GetSprite))
  (Character|LaunchCharacter _returnvalue "0.000000, 0,600.000000" false true)
  (bind _as2dside_scroller_character (Utilities|Casting|CastTo2DSideScrollerCharacter _returnvalue))
  (Utilities|FlowControl|MultiGate false false -1
    (:Out%200
      (Sprite|SetFlipbook _sprite "/Game/Truelle/Truele2.Truele2"))
    (:Out%201
      (Sprite|SetFlipbook _sprite "/Game/Truelle/TRuelle3.TRuelle3"))
    (:Out%202
      (Sprite|SetFlipbook _sprite "/Game/Truelle/TruelleCheckpoinFinalt.TruelleCheckpoinFinalt")
      (Utilities|FlowControl|DoOnce false
        (:Completed
          (Variables|/Game/2DSideScrollerBP/Blueprints/2DSideScrollerCharacter.2DSideScrollerCharacter_C|SetSpawnJoueur _as2dside_scroller_character (Math|Vector|MakeVector (.x _respawnpos) 0.0 (.z _respawnpos)))
          (Components|DestroyComponent (Variables|Default|GetBox))
          (Utilities|FlowControl|Delay 2.0)
          (Sprite|SetFlipbook (Variables|Default|GetSprite) "/Game/Truelle/Truelle4.Truelle4"))))))

(event EventBeginPlay
  (Variables|Default|SetRespawnPos (Transformation|GetWorldLocation (Variables|Default|GetBox))))

(event Collision|EventActorBeginOverlap
  (params (OtherActor :type Actor%20Object%20Reference)))

(event EventTick
  (params (DeltaSeconds :type Float%20%28single-precision%29)))

(fn ConstructionScript)